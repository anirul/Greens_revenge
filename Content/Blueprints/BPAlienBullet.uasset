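; BPAlienBullet is an alien projectile actor that cleans itself up when it expires or leaves the play area.
; BeginPlay starts a fixed-delay lifetime timer, while Tick destroys it once its SphereCollision strays too far from the world origin on X or Y.
; The graph holds no movement or hit logic, as the overlap event is a disabled stub.
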(event `self.ReceiveBeginPlay`
  (`KismetSystemLibrary.Delay` 10.0)
  (`self.K2_DestroyActor`))

(event `self.ReceiveTick`
  (params (DeltaSeconds :type "Float (single-precision)"))
  (if (or (> (`KismetMathLibrary.Abs` (.x (`SceneComponent.K2_GetComponentLocation` (`self.SphereCollision`)))) 5000.0) (> (`KismetMathLibrary.Abs` (.y (`SceneComponent.K2_GetComponentLocation` (`self.SphereCollision`)))) 5000.0))
    (`self.K2_DestroyActor`)))

(fn `UserConstructionScript`)