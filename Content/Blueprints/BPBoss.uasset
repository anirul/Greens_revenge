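; Boss enemy actor for a shooter that fires alien bullets in eight directions and dies after enough player bullet hits.
; Tick accumulates time and calls FireEverywhere, which spawns a BPAlienBullet at each directional arrow component whenever the fire-rate interval has elapsed.
; Overlapping player bullets are destroyed and reduce BossLife; at zero the boss spawns an explosion, adds to the player pawn's EnemyDead tally and destroys itself.
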(event `self.ReceiveActorBeginOverlap`
  (params (OtherActor :type "Actor Object Reference"))
  (bind _asbpplayer_bullet (cast `/Game/Blueprints/BPPlayerBullet` OtherActor))
  (bind _output_get (set `self.BossLife` (- (`self.BossLife`) 1)))
  (`self.K2_DestroyActor` _asbpplayer_bullet)
  (if (<= _output_get 0)
    (`|SpawnActorFromClass` "/Game/StarterContent/Blueprints/Blueprint_Effect_Explosion.Blueprint_Effect_Explosion_C" (`self.GetTransform`) "Undefined" "OverrideRootScale")
    (bind _asbpplayer_pawn (cast `/Game/Blueprints/BPPlayerPawn` (`GameplayStatics.GetPlayerPawn` 0))
      (:`then`
        (set `/Game/Blueprints/BPPlayerPawn.EnemyDead` (+ (`/Game/Blueprints/BPPlayerPawn.EnemyDead` _asbpplayer_pawn) 100) _asbpplayer_pawn))
      (:`CastFailed`
        _))
    (`self.K2_DestroyActor`)))

(event `self.ReceiveTick`
  (params (DeltaSeconds :type "Float (single-precision)"))
  (set `self.TimeAcc` (+ (`self.TimeAcc`) DeltaSeconds))
  (`self.FireEverywhere`))

(fn `FireEverywhere`
  (if (> (- (`self.TimeAcc`) (`self.LastTimeFire`)) (`self.BossRateOfFire`))
    ;[1 1 1] Fire!
    (`|SpawnActorFromClass` "/Game/Blueprints/BPAlienBullet.BPAlienBullet_C" (`SceneComponent.K2_GetComponentToWorld` (`self.ArrowLeft`)) "AlwaysSpawn" "OverrideRootScale")
    (`|SpawnActorFromClass` "/Game/Blueprints/BPAlienBullet.BPAlienBullet_C" (`SceneComponent.K2_GetComponentToWorld` (`self.ArrowRight`)) "AlwaysSpawn" "OverrideRootScale")
    (`|SpawnActorFromClass` "/Game/Blueprints/BPAlienBullet.BPAlienBullet_C" (`SceneComponent.K2_GetComponentToWorld` (`self.ArrowUp`)) "AlwaysSpawn" "OverrideRootScale")
    (`|SpawnActorFromClass` "/Game/Blueprints/BPAlienBullet.BPAlienBullet_C" (`SceneComponent.K2_GetComponentToWorld` (`self.ArrowDown`)) "AlwaysSpawn" "OverrideRootScale")
    (`|SpawnActorFromClass` "/Game/Blueprints/BPAlienBullet.BPAlienBullet_C" (`SceneComponent.K2_GetComponentToWorld` (`self.ArrowUpLeft`)) "AlwaysSpawn" "OverrideRootScale")
    (`|SpawnActorFromClass` "/Game/Blueprints/BPAlienBullet.BPAlienBullet_C" (`SceneComponent.K2_GetComponentToWorld` (`self.ArrowUpRight`)) "AlwaysSpawn" "OverrideRootScale")
    (`|SpawnActorFromClass` "/Game/Blueprints/BPAlienBullet.BPAlienBullet_C" (`SceneComponent.K2_GetComponentToWorld` (`self.ArrowDownLeft`)) "AlwaysSpawn" "OverrideRootScale")
    (`|SpawnActorFromClass` "/Game/Blueprints/BPAlienBullet.BPAlienBullet_C" (`SceneComponent.K2_GetComponentToWorld` (`self.ArrowDownRight`)) "AlwaysSpawn" "OverrideRootScale")
    (set `self.LastTimeFire` (`self.TimeAcc`))))

(fn `UserConstructionScript`)