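; Player pawn for a ship that moves forward and turns in yaw under player input.
; MoveSide sets the turn rate, while ChangeSpeed scales a base forward speed around its neutral value, so zero input still moves the ship.
; Tick applies both, scaled by delta time: a swept location step from the Sphere along the Arrow's forward vector, then a yaw change that preserves pitch and roll.
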(event `self.ReceiveTick`
  (params (DeltaSeconds :type "Float (single-precision)"))
  (`self.SetShipMove` DeltaSeconds (`self.Forward player`))
  (`self.SetShipRotation` DeltaSeconds (`self.Rotation player`)))

(event `InputAxis|MoveSide`
  (params (AxisValue :type "Float (single-precision)"))
  ;[1 1 1] Rotation changed by player
  (set `self.Rotation player` (* (`self.Rotation Move Inc`) AxisValue)))

(event `InputAxis|ChangeSpeed`
  (params (AxisValue :type "Float (single-precision)"))
  ;[1 1 1] Forward speed changed by player
  (set `self.Forward player` (* (`self.Forward Move Inc`) (+ (* AxisValue 0.5) 1.0))))

(fn `SetShipMove`
  (params (deltaT :type "Float (double-precision)") (ForwardMove :type "Float (double-precision)"))
  (`self.K2_SetActorLocation` (+ (`SceneComponent.K2_GetComponentLocation` (`self.Sphere`)) (* (`KismetMathLibrary.Normal` (`SceneComponent.GetForwardVector` (`self.Arrow`))) (* deltaT ForwardMove))) true))

(fn `SetShipRotation`
  (params (DeltaT :type "Float (double-precision)") (`Rotation Move` :type "Float (double-precision)"))
  (`self.K2_SetActorRotation` (`KismetMathLibrary.MakeRotator` (.roll (`self.K2_GetActorRotation`)) (.pitch (`self.K2_GetActorRotation`)) (+ (* DeltaT `Rotation Move`) (.yaw (`self.K2_GetActorRotation`))))))

(fn `UserConstructionScript`)