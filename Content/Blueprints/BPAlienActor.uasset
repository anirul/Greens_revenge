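; BPAlienActor is an enemy alien that chases the player pawn and shoots at it.
; Each Tick it moves toward the player in X and Y with a swept move, keeping its own Z, and rotates to face them.
; It accumulates time to fire a BPAlienBullet from its Arrow at a set interval.
; Overlapping a player bullet or the player pawn decrements the player's enemy count, triggers DogeShout, then spawns an explosion and destroys the alien.
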(event `self.ReceiveActorBeginOverlap`
  (params (OtherActor :type "Actor Object Reference"))
  (cast `/Game/Blueprints/BPPlayerBullet` OtherActor
    (:`then`
      _)
    (:`CastFailed`
      (cast `/Game/Blueprints/BPPlayerPawn` OtherActor)))
  (bind _asbpplayer_pawn (cast `/Game/Blueprints/BPPlayerPawn` (`GameplayStatics.GetPlayerPawn` 0)))
  (`/Game/Blueprints/BPPlayerPawn.DecreaseEnemy` _asbpplayer_pawn)
  (`/Game/Blueprints/BPPlayerPawn.Doge shout` _asbpplayer_pawn)
  (`self.Explode`))

(event `self.ReceiveTick`
  (params (DeltaSeconds :type "Float (single-precision)"))
  (set `self.TimeAcc` (+ (`self.TimeAcc`) DeltaSeconds))
  (`self.GoToPlayer` DeltaSeconds)
  (`self.ShootAtPlayer`))

(fn `Explode`
  (`|SpawnActorFromClass` "/Game/StarterContent/Blueprints/Blueprint_Effect_Explosion.Blueprint_Effect_Explosion_C" (`self.GetTransform`) "Undefined" "OverrideRootScale")
  (`self.K2_DestroyActor`))

(fn `GoToPlayer`
  (params (DeltaT :type "Float (double-precision)"))
  (bind _returnvalue (`self.K2_GetActorLocation`))
  (bind _returnvalue_2 (`SceneComponent.K2_GetComponentLocation` (`self.SphereCollision`)))
  (bind _returnvalue_3 (`self.K2_GetActorLocation` (`GameplayStatics.GetPlayerPawn` 0)))
  (`self.K2_SetActorLocationAndRotation` (`KismetMathLibrary.MakeVector` (.x (+ _returnvalue_2 (* (* (`KismetMathLibrary.Normal` (- _returnvalue_3 _returnvalue)) DeltaT) (`self.EnemySpeed`)))) (.y (+ _returnvalue_2 (* (* (`KismetMathLibrary.Normal` (- _returnvalue_3 _returnvalue)) DeltaT) (`self.EnemySpeed`)))) (.z _returnvalue_2)) (`KismetMathLibrary.FindLookAtRotation` _returnvalue _returnvalue_3) true))

(fn `ShootAtPlayer`
  (if (> (- (`self.TimeAcc`) (`self.LastTimeFire`)) (`self.EnemyRateOdFire`))
    (`|SpawnActorFromClass` "/Game/Blueprints/BPAlienBullet.BPAlienBullet_C" (`SceneComponent.K2_GetComponentToWorld` (`self.Arrow`)) "AlwaysSpawn" "OverrideRootScale")
    (set `self.LastTimeFire` (`self.TimeAcc`))))

(fn `UserConstructionScript`)